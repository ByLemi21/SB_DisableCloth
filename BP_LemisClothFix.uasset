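; BP_LemisClothFix is a component that turns off cloth simulation on its owner's skeletal mesh while the game is paused.
; On BeginPlay it caches the owner's SkeletalMeshComponent.
; Every Tick it polls the pause state, setting cloth blend weight to zero and suspending simulation when paused, and restoring full weight and resuming it otherwise.
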(event `self.ReceiveBeginPlay`
  (bind _returnvalue (`Actor.GetComponentByClass` (`self.GetOwner`) "/Script/Engine.SkeletalMeshComponent"))
  (`/Engine/EditorBlueprintResources/StandardMacros.IsValid` _returnvalue
    (:`Is Valid`
      (set `self.SkelMeshComp` _returnvalue))))

(event `self.ReceiveTick`
  (params (DeltaSeconds :type "Float (single-precision)"))
  (bind _skelmeshcomp (`self.SkelMeshComp`))
  (`/Engine/EditorBlueprintResources/StandardMacros.IsValid` _skelmeshcomp
    (:`Is Valid`
      (if (`GameplayStatics.IsGamePaused`)
        (set `SkeletalMeshComponent.ClothBlendWeight` 0.0 _skelmeshcomp)
        (`SkeletalMeshComponent.SuspendClothingSimulation` _skelmeshcomp)
        (else
          (set `SkeletalMeshComponent.ClothBlendWeight` 1.0 _skelmeshcomp)
          (`SkeletalMeshComponent.ResumeClothingSimulation` _skelmeshcomp))))))